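; VR player that spawns and drives a separate IK_Pawn as its full-body IK avatar.
; BeginPlay links NetAvatar to the first NetClient and spawns the pawn; the IK_Camera and possession branch is disabled.
; Tick moves and turns the pawn from input axes, writes tracking-space controller and HMD poses as its child components' world transforms, and tints the body by NetID hue.
; Copying poses to NetAvatar is left unconnected.
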(event EventBeginPlay
  (bind _self self)
  (Utilities|FlowControl|Sequence
    (:then_0
      (bind _outactors (Actor|GetAllActorsOfClass "/Script/DynamicalSystems.NetClient"))
      (Variables|/Script/DynamicalSystems.NetAvatar|SetNetClient (Variables|Default|GetNetAvatar) (Utilities|Array|Get(acopy) _outactors)))
    (:then_1
      (bind _returnvalue (Game|SpawnActorfromClass "/Game/FullBodyIK/Blueprints/IK_Pawn.IK_Pawn_C" (Transformation|GetWorldTransform (Variables|Default|GetTransformComponent)) "AlwaysSpawn" 0 0))
      (bind _asik_pawn (Utilities|Casting|CastToIK_Pawn _returnvalue))
      (bind _output_get (Variables|Default|SetIK_Pawn _asik_pawn))
      (if (not true)
        (bind _returnvalue_2 (Game|SpawnActorfromClass "/Game/FullBodyIK/Blueprints/IK_Camera.IK_Camera_C" (Math|Transform|ComposeTransforms (Transformation|GetWorldTransform (Variables|/Game/FullBodyIK/Blueprints/IK_Pawn.IK_Pawn_C|GetVROrigin _output_get)) (Math|Transform|MakeTransform "0, 0, 0")) "AlwaysSpawn" 0 0))
        (bind _output_get_2 (Variables|Default|SetIK_Camera _returnvalue_2))
        (Game|Player|SetViewTargetwithBlend _self _output_get_2 0.0 "VTBlend_Linear" 0.0 false)
        (Pawn|Possess _self _returnvalue)))))

(event EventTick
  (params (DeltaSeconds :type Float%20%28single-precision%29))
  (bind (_devicerotation _deviceposition) (Class|HeadMountedDisplayFunctionLibrary|GetOrientationandPosition))
  (bind _ik_pawn (Variables|Default|GetIK_Pawn))
  (bind _ik_pawn_2 (Variables|Default|GetIK_Pawn))
  (bind _defaultsceneroot (Variables|/Game/FullBodyIK/Blueprints/IK_Pawn.IK_Pawn_C|GetDefaultSceneRoot _ik_pawn))
  (Utilities|IsValid _ik_pawn_2
    (:Is%20Valid
      (Utilities|FlowControl|Sequence
        (:then_0
          ;[1 1 1] Motion Controlled Locomotion
          (Transformation|SetWorldLocation _defaultsceneroot (+ (Transformation|GetWorldLocation _defaultsceneroot) (+ (* (Math|Vector|GetRightVector _defaultsceneroot) (* DeltaSeconds (* (Input|AxisValues|GetMoveForward) -1e+02))) (* (Math|Vector|GetForwardVector _defaultsceneroot) (* DeltaSeconds (* (Input|AxisValues|GetMoveSide) -1e+02))))) false false)
          (Transformation|SetWorldRotation (Variables|/Game/FullBodyIK/Blueprints/IK_Pawn.IK_Pawn_C|GetDefaultSceneRoot (Variables|Default|GetIK_Pawn)) (Math|Rotator|CombineRotators (Transformation|GetWorldRotation _defaultsceneroot) (Math|Rotator|MakeRotator 0.0 0.0 (* (Input|AxisValues|GetRotate) 1.0))) false false))
        (:then_1
          (Transformation|SetWorldTransform (Variables|/Game/FullBodyIK/Blueprints/IK_Pawn.IK_Pawn_C|GetChildMotionControllerL (Variables|Default|GetIK_Pawn)) (Transformation|GetRelativeTransform (Variables|Default|GetMotionControllerL)) false false)
          (Transformation|SetWorldTransform (Variables|/Game/FullBodyIK/Blueprints/IK_Pawn.IK_Pawn_C|GetChildMotionControllerR (Variables|Default|GetIK_Pawn)) (Transformation|GetRelativeTransform (Variables|Default|GetMotionControllerR)) false false)
          (Transformation|SetWorldTransform (Variables|/Game/FullBodyIK/Blueprints/IK_Pawn.IK_Pawn_C|GetChildHMD (Variables|Default|GetIK_Pawn)) (Math|Transform|MakeTransform _deviceposition _devicerotation "1,1,1") false false))
        (:then_3
          (Default|SetBodyColor _ik_pawn_2 (Class|KismetMathLibrary|HSVtoRGB (/ (Math|Conversions|ToFloat(Integer) (Variables|/Script/DynamicalSystems.NetAvatar|GetNetID (Variables|Default|GetNetAvatar))) 2e+01) 0.7 0.5 1.0)))))))

(fn ConstructionScript)